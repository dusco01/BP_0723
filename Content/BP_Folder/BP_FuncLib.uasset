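; BP_FuncLib is a Blueprint function library of small arithmetic and debug-print utilities, apparently practice functions.
; Multi and Divide return the product and the floating-point quotient of two inputs.
; Print, MultiArr and OddEven print, respectively, a number range, formatted times tables over a range, and a Korean even-or-odd label.
; HelloWorld prints a fixed greeting.
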(fn Multi
  (params (A :type Integer) (B :type Integer))
  (return (* A B)))

(fn Print
  (params (A :type Integer) (B :type Integer))
  (for _index (range A B)
    (Development|PrintString 0 (Utilities|String|ToString(Integer) _index))))

(fn HelloWorld
  (Development|PrintString 0 "Hello World"))

(fn MultiArr
  (params (A :type Integer) (B :type Integer))
  (for _index (range A B)
    (for _index_2 (range 1 9)
      (Development|PrintText 0 (Utilities|Text|FormatText "{0} * {1} = {2}" _index _index_2 (* _index _index_2)) true true "(R=0.000000,G=0.660000,B=1.000000,A=1.000000)" 999.0))))

(fn Divide
  (params (A :type Integer) (B :type Integer))
  (return (/ (Math|Conversions|ToFloat(Integer) A) (Math|Conversions|ToFloat(Integer) B))))

(fn OddEven
  (params (A :type Integer))
  (if (== (Math|Integer|%(Integer) A 2) 0)
    (Development|PrintString 0 "짝수")
    (else
      (Development|PrintString 0 "홀수"))))