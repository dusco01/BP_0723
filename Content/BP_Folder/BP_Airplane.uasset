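; Airplane actor that flies forward along its forward vector every Tick at Speed, without sweep.
; LeftRotation and RightRotation input axes both add local pitch to StaticMesh, scaled by RotateSpeed.
; BeginPlay also runs a by-reference Swap test on A and B and prints the result, unrelated to flight.
; An unconnected NewFunction print is left in the graph.
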(event EventBeginPlay
  (CallFunction|Swap (Variables|Default|GetA) (Variables|Default|GetB))
  (Development|PrintString (Utilities|String|ToString(Text) (Utilities|Text|FormatText "A = {0}, B = {1}" (Variables|Default|GetA) (Variables|Default|GetB))) true true "(R=0.000000,G=0.660000,B=1.000000,A=1.000000)" 999.0))

(event EventTick
  (params (DeltaSeconds :type Float%20%28single-precision%29))
  (Transformation|SetActorLocation (+ (Transformation|GetActorLocation) (* (Transformation|GetActorForwardVector) (* DeltaSeconds (Variables|Default|GetSpeed)))) false false))

(event Input|AxisEvents|InputAxisLeftRotation
  (params (AxisValue :type Float%20%28single-precision%29))
  (Transformation|AddLocalRotation (Variables|Default|GetStaticMesh) (Math|Rotator|MakeRotator 0.0 (* AxisValue (Variables|Default|GetRotateSpeed)) 0.0) false false))

(event Input|AxisEvents|InputAxisRightRotation
  (params (AxisValue :type Float%20%28single-precision%29))
  (Transformation|AddLocalRotation (Variables|Default|GetStaticMesh) (Math|Rotator|MakeRotator 0.0 (* AxisValue (Variables|Default|GetRotateSpeed)) 0.0) false false))

(fn ConstructionScript)

(fn Swap
  (params (A :type Integer%20%28by%20ref%29) (B :type Integer%20%28by%20ref%29))
  (bind _output_get (LocalVariables|SetC A))
  (|SetBy-RefVar A B)
  (|SetBy-RefVar B _output_get)
  (Development|PrintString ""))