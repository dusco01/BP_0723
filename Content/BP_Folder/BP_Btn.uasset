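; BP_Btn is a pressure-style button that moves a referenced Target actor while the player overlaps it.
; Begin and end overlap events on the Btn component toggle the IsClick flag, responding only to BP_Player.
; While the flag is set, Tick shifts Target along world +X by a fixed, frame-rate-dependent step.
; An unconnected node chain for moving Target back along -X never runs.
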(event OnComponentBeginOverlap(Btn)
  (params (OverlappedComponent :type Primitive%20Component%20Object%20Reference) (OtherActor :type Actor%20Object%20Reference) (OtherComp :type Primitive%20Component%20Object%20Reference) (OtherBodyIndex :type Integer) (bFromSweep :type Boolean) (SweepResult :type Hit%20Result%20Structure%20%28by%20ref%29))
  (Utilities|Casting|CastToBP_Player OtherActor)
  (Variables|Default|SetIsClick true))

(event OnComponentEndOverlap(Btn)
  (params (OverlappedComponent :type Primitive%20Component%20Object%20Reference) (OtherActor :type Actor%20Object%20Reference) (OtherComp :type Primitive%20Component%20Object%20Reference) (OtherBodyIndex :type Integer))
  (Utilities|Casting|CastToBP_Player OtherActor)
  (Variables|Default|SetIsClick false))

(event EventTick
  (params (DeltaSeconds :type Float%20%28single-precision%29))
  (bind _target (Variables|Default|GetTarget))
  (bind _returnvalue (Transformation|GetActorLocation _target))
  (if (Variables|Default|GetIsClick)
    (Transformation|SetActorLocation (Variables|Default|GetTarget) (Math|Vector|MakeVector (+ (.x _returnvalue) 1e+01) (.y _returnvalue) (.z _returnvalue)) false false)))

(fn ConstructionScript)